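; BP_Actor1 is an actor that moves in the horizontal plane at a set direction and speed, bouncing off whatever it hits.
; Each tick it does a swept world offset; on a blocking hit it reflects Direction around the surface normal.
; Each bounce subtracts a fixed deceleration, a tenth of the starting speed, clamped to MinSpeed, and prints the new speed for debugging.
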(event EventBeginPlay
  (Variables|Default|SetDeceleration (* (Variables|Default|GetSpeed) 0.1)))

(event EventTick
  (params (DeltaSeconds :type Float%20%28single-precision%29))
  (bind _sweephitresult (Transformation|AddActorWorldOffset (Math|Vector|MakeVector (.x (* (* (Variables|Default|GetDirection) (Variables|Default|GetSpeed)) DeltaSeconds)) (.y (* (* (Variables|Default|GetDirection) (Variables|Default|GetSpeed)) DeltaSeconds)) 0.0) true))
  (if (.bBlockingHit (Collision|BreakHitResult _sweephitresult))
    (Variables|Default|SetDirection (Math|Vector|GetReflectionVector (Variables|Default|GetDirection) (.Normal (Collision|BreakHitResult _sweephitresult))))
    (Variables|Default|SetSpeed (Math|Float|Max(Float) (- (Variables|Default|GetSpeed) (Variables|Default|GetDeceleration)) (Variables|Default|GetMinSpeed)))
    (Development|PrintString (Utilities|String|ToString(Float) (Variables|Default|GetSpeed)) true true "(R=0.000000,G=1.000000,B=0.229393,A=1.000000)")))

(fn ConstructionScript)